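; Tunnel segment for an endless-tunnel game: when the player reaches its trigger, it has TunnelSpawner spawn another, adds score and destroys itself.
; RandomizeWall picks a holed wall mesh and roll, then keeps either an enemy (about 90%) or an HP pack.
; Tick spins the wall and jitters the enemy.
; Collisions handle player damage and healing, projectiles blocked by walls, and enemy kills that award score.
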(event `self.ReceiveTick`
  (params (DeltaSeconds :type "Float (single-precision)"))
  (bind _wallmesh (`self.WallMesh`))
  (bind _tunnel_enemy (`self.Tunnel_Enemy`))
  (if (`KismetSystemLibrary.IsValid` _wallmesh)
    (`SceneComponent.K2_AddLocalRotation` _wallmesh (`KismetMathLibrary.MakeRotator` (* DeltaSeconds (`self.RotateSpeed`))) false false)
    (`/Engine/EditorBlueprintResources/StandardMacros.IsValid` _tunnel_enemy
      (:`Is Valid`
        (`SceneComponent.K2_AddLocalOffset` _tunnel_enemy (* (`KismetMathLibrary.RandomUnitVector`) (10.0 10.0 10.0)) true false)))))

(event `self.TriggerZone.OnComponentBeginOverlap`
  (params (OverlappedComponent :type "PrimitiveComponent Object Reference") (OtherActor :type "Actor Object Reference") (OtherComp :type "PrimitiveComponent Object Reference") (OtherBodyIndex :type Integer) (bFromSweep :type Boolean) (SweepResult :type "HitResult Structure (by ref)"))
  (bind _asbp_player (cast `/Game/InfiniteMatrix/Blueprints/BP_Player` OtherActor))
  (`/Game/InfiniteMatrix/Blueprints/BP_TunnelSpawner.SpawnTunnelAtSpawnPoint` (`self.TunnelSpawner`))
  (set `/Game/InfiniteMatrix/Blueprints/BP_Player.MyScore` (+ (`/Game/InfiniteMatrix/Blueprints/BP_Player.MyScore` _asbp_player) 1) _asbp_player)
  (`self.K2_DestroyActor`))

(event `self.WallMesh.OnComponentHit`
  (params (HitComponent :type "PrimitiveComponent Object Reference") (OtherActor :type "Actor Object Reference") (OtherComp :type "PrimitiveComponent Object Reference") (NormalImpulse :type "Vector Structure") (Hit :type "HitResult Structure (by ref)"))
  (`ActorComponent.K2_DestroyComponent` HitComponent)
  (bind _asbp_player (cast `/Game/InfiniteMatrix/Blueprints/BP_Player` OtherActor))
  (`/Engine/EditorBlueprintResources/StandardMacros.IsValid` _asbp_player
    (:`Is Valid`
      (`/Game/InfiniteMatrix/Blueprints/BP_Player.DecrementHP` _asbp_player))))

(event `self.HPPack.OnComponentHit`
  (params (HitComponent :type "PrimitiveComponent Object Reference") (OtherActor :type "Actor Object Reference") (OtherComp :type "PrimitiveComponent Object Reference") (NormalImpulse :type "Vector Structure") (Hit :type "HitResult Structure (by ref)"))
  (`ActorComponent.K2_DestroyComponent` HitComponent)
  (bind _asbp_player (cast `/Game/InfiniteMatrix/Blueprints/BP_Player` OtherActor))
  (`/Game/InfiniteMatrix/Blueprints/BP_Player.IncrementHP` _asbp_player))

(event `self.WallMesh.OnComponentBeginOverlap`
  (params (OverlappedComponent :type "PrimitiveComponent Object Reference") (OtherActor :type "Actor Object Reference") (OtherComp :type "PrimitiveComponent Object Reference") (OtherBodyIndex :type Integer) (bFromSweep :type Boolean) (SweepResult :type "HitResult Structure (by ref)"))
  (cast `/Game/InfiniteMatrix/Blueprints/Player_Projectile` OtherActor)
  (`self.K2_DestroyActor` OtherActor))

(event `self.EnemyHitBox.OnComponentBeginOverlap`
  (params (OverlappedComponent :type "PrimitiveComponent Object Reference") (OtherActor :type "Actor Object Reference") (OtherComp :type "PrimitiveComponent Object Reference") (OtherBodyIndex :type Integer) (bFromSweep :type Boolean) (SweepResult :type "HitResult Structure (by ref)"))
  (bind _asplayer_projectile (cast `/Game/InfiniteMatrix/Blueprints/Player_Projectile` OtherActor)
    (:`then`
      (`/Engine/EditorBlueprintResources/StandardMacros.IsValid` _asplayer_projectile
        (:`Is Valid`
          (`/Game/InfiniteMatrix/Blueprints/BP_Player.IncrementScore` (`/Game/InfiniteMatrix/Blueprints/Player_Projectile.Proj_Player_ref` _asplayer_projectile))
          (`self.K2_DestroyActor` OtherActor))))
    (:`CastFailed`
      (bind _asbp_player (cast `/Game/InfiniteMatrix/Blueprints/BP_Player` OtherActor))
      (`/Engine/EditorBlueprintResources/StandardMacros.IsValid` _asbp_player
        (:`Is Valid`
          (`/Game/InfiniteMatrix/Blueprints/BP_Player.DecrementHP` _asbp_player)))))
  (`ActorComponent.K2_DestroyComponent` (`self.Eye1`))
  (`ActorComponent.K2_DestroyComponent` (`self.Eye2`))
  (`ActorComponent.K2_DestroyComponent` (`self.Head`))
  (`ActorComponent.K2_DestroyComponent` (`self.SpotLight`))
  (`ActorComponent.K2_DestroyComponent` (`self.EnemyHitBox`))
  (`ActorComponent.K2_DestroyComponent` (`self.Tunnel_Enemy`)))

(fn `RandomizeWall`
  (bind _tunnel_enemy (`self.Tunnel_Enemy`))
  (`StaticMeshComponent.SetStaticMesh` (`self.WallMesh`) (select `int` (`KismetMathLibrary.RandomIntegerInRange` 0 3) :`0` "/Game/InfiniteMatrix/Meshes/SM_Hole_01.SM_Hole_01" :`1` "/Game/InfiniteMatrix/Meshes/SM_Hole_02.SM_Hole_02" :`2` "/Game/InfiniteMatrix/Meshes/SM_Hole_03.SM_Hole_03" :`3` "/Game/InfiniteMatrix/Meshes/SM_Hole_04.SM_Hole_04" :!type "StaticMesh Object Reference"))
  (`SceneComponent.K2_AddLocalRotation` (`self.WallMesh`) (`KismetMathLibrary.MakeRotator` (`KismetMathLibrary.RandomFloatInRange` 0.0 360.0)) false false)
  (`/Engine/EditorBlueprintResources/StandardMacros.CompareFloat` (`KismetMathLibrary.RandomFloat`) 0.1
    (:`>`
      (`ActorComponent.K2_DestroyComponent` (`self.HPPack`))
      (`SceneComponent.K2_AddLocalOffset` _tunnel_enemy (0.0 0.0 0.0) false false)
      (`SceneComponent.K2_AddLocalRotation` _tunnel_enemy (`KismetMathLibrary.MakeRotator` 0.0 0.0 90.0) false false))
    (:`==`
      (`SceneComponent.K2_AddLocalOffset` (`self.HPPack`) (`KismetMathLibrary.MakeVector` (`KismetMathLibrary.RandomFloatInRange` -25.0 25.0) (`KismetMathLibrary.RandomFloatInRange` -25.0 25.0) (`KismetMathLibrary.RandomFloatInRange` -25.0 25.0)) false false :!label _label)
      (`ActorComponent.K2_DestroyComponent` (`self.Eye1`))
      (`ActorComponent.K2_DestroyComponent` (`self.Eye2`))
      (`ActorComponent.K2_DestroyComponent` (`self.Head`))
      (`ActorComponent.K2_DestroyComponent` (`self.SpotLight`))
      (`ActorComponent.K2_DestroyComponent` (`self.EnemyHitBox`))
      (`ActorComponent.K2_DestroyComponent` (`self.Tunnel_Enemy`)))
    (:`<`
      (goto _label))))

(fn `UserConstructionScript`)