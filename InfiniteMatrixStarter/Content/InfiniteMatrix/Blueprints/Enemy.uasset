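; Enemy actor that damages the player on impact and is destroyed by hits or overlaps with its sphere.
; Any sphere hit destroys it; a BP_Player hit also loses HP, flagged dead with a restart display at zero.
; Any sphere overlap also destroys it, and removes the root component of an overlapping Player_Projectile.
; SpawnEnemy shifts the root by a fixed X and random Y/Z offset, then rotates it, ignoring TunnelPos.
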(event `self.EnemyBox.OnComponentHit`
  (params (HitComponent :type "PrimitiveComponent Object Reference") (OtherActor :type "Actor Object Reference") (OtherComp :type "PrimitiveComponent Object Reference") (NormalImpulse :type "Vector Structure") (Hit :type "HitResult Structure (by ref)")))

(event `self.Sphere.OnComponentHit`
  (params (HitComponent :type "PrimitiveComponent Object Reference") (OtherActor :type "Actor Object Reference") (OtherComp :type "PrimitiveComponent Object Reference") (NormalImpulse :type "Vector Structure") (Hit :type "HitResult Structure (by ref)"))
  (`self.K2_DestroyActor` self)
  (bind _asbp_player (cast `/Game/InfiniteMatrix/Blueprints/BP_Player` OtherActor))
  (`/Engine/EditorBlueprintResources/StandardMacros.IsValid` _asbp_player
    (:`Is Valid`
      (`/Game/InfiniteMatrix/Blueprints/BP_Player.DecrementHP` _asbp_player)
      (`/Engine/EditorBlueprintResources/StandardMacros.CompareInt` (`/Game/InfiniteMatrix/Blueprints/BP_Player.MyHP` _asbp_player)
        (:`==`
          (set `/Game/InfiniteMatrix/Blueprints/BP_Player.IsDead` true _asbp_player)
          (`/Game/InfiniteMatrix/Blueprints/BP_Player.DisplayRestart` _asbp_player))))))

(event `self.Sphere.OnComponentBeginOverlap`
  (params (OverlappedComponent :type "PrimitiveComponent Object Reference") (OtherActor :type "Actor Object Reference") (OtherComp :type "PrimitiveComponent Object Reference") (OtherBodyIndex :type Integer) (bFromSweep :type Boolean) (SweepResult :type "HitResult Structure (by ref)"))
  (`self.K2_DestroyActor` self)
  (bind _asplayer_projectile (cast `/Game/InfiniteMatrix/Blueprints/Player_Projectile` OtherActor))
  (`/Engine/EditorBlueprintResources/StandardMacros.IsValid` _asplayer_projectile
    (:`Is Valid`
      (`ActorComponent.K2_DestroyComponent` (`Actor.RootComponent` OtherActor)))))

(fn `SpawnEnemy`
  (params (TunnelPos :type "Vector Structure"))
  (`SceneComponent.K2_AddLocalOffset` (`self.DefaultSceneRoot`) (`KismetMathLibrary.MakeVector` -300.0 (`KismetMathLibrary.RandomFloatInRange` -300.0 300.0) (`KismetMathLibrary.RandomFloatInRange` -300.0 300.0)) true false)
  (`SceneComponent.K2_AddLocalRotation` (`self.DefaultSceneRoot`) (struct :`Yaw` 90.0) false false))

(fn `UserConstructionScript`)